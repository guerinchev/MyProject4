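; Game mode for a Pac-Man game that runs the intro, score, lives, power-pellet state and audio.
; Input is disabled during intro music, then enemies are activated and possessed.
; A timed NeedsToRun flag drives fleeing audio, while Tick mutes background noise during fleeing or death.
; Player destruction triggers a delayed respawn that rebinds the destroy event; exhausted lives or cleared pellets open the end screen.
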(event `PowerPelletAudio`
  ;[1 1 1] Power Pellet Audio
  (`self.EnemyRunningAwayAudio`))

(event `EnemyRunningAwayAudio`
  (bind _enemyrunningawaynoise (`self.EnemyRunningAwayNoise`))
  ;[1 1 1] Enemy Running Away Audio
  (if (== (`self.NeedsToRun`) (`self.True`))
    (if (not (`ActorComponent.IsActive` _enemyrunningawaynoise))
      (`ActorComponent.Activate` _enemyrunningawaynoise false)
      (`KismetSystemLibrary.Delay` 8.0)))
  (`ActorComponent.Deactivate` _enemyrunningawaynoise))

(event `PlayIntroMusic`
  (bind _intromusic (`self.IntroMusic`))
  ;[1 1 1] Play Intro Music
  (`self.DisablePlayerInput`)
  (if (< _intromusic 1)
    (`GameplayStatics.PlaySound2D` "/Game/audio/pacman_intro_music.pacman_intro_music" 1.0 1.0 0.0 null null)
    (`KismetSystemLibrary.Delay` 4.5)
    (`ActorComponent.Activate` (`self.PacmanBackgroundNoise`) false)
    (set `self.IntroMusic` (+ _intromusic 1))
    (`self.ActivateEnemiesAndPlayersMovement`)
    (`self.EnablePlayerInput`)))

(event `self.ReceiveTick`
  (params (DeltaSeconds :type "Float (single-precision)"))
  ;[1 1 1] Play Background Noise
  (if (or (`self.NeedsToRun`) (`self.PacmanDied`))
    (`ActorComponent.Deactivate` (`self.PacmanBackgroundNoise`))
    (elif (and (== (`self.IntroMusic`) 1) (`|EnumEquality` (`AudioComponent.GetPlayState` (`self.PacmanBackgroundNoise`)) "Stopped"))
      (`ActorComponent.Activate` (`self.PacmanBackgroundNoise`) false))))

(event `AddPelletPoints`
  (params (AddPoint :type Integer))
  ;[1 1 1] Score
  (set `self.Score` (+ AddPoint (`self.Score`)))
  (bind _outactors (`GameplayStatics.GetAllActorsOfClass` "/Game/objects/powerPellets.powerPellets_C"))
  (bind _outactors_2 (`GameplayStatics.GetAllActorsOfClass` "/Game/objects/normalPellets.normalPellets_C"))
  (if (and (== (`KismetArrayLibrary.Array_Length` _outactors_2) 0) (== 0 (`KismetArrayLibrary.Array_Length` _outactors)))
    (`GameplayStatics.OpenLevel` (`self.EndScreen`))))

(event `EatingGhostPoints`
  (params (`Add Points` :type Integer))
  ;[1 1 1] Add Ghost Eaten Points
  (set `self.Score` (+ `Add Points` (`self.Score`))))

(event `PowerPelletTimer`
  (params (`Eaten Pellet` :type Boolean))
  ;[1 1 1] Power Pellet Time to Last
  (if `Eaten Pellet`
    (set `self.NeedsToRun` true)
    (`KismetSystemLibrary.Delay` (`KismetMathLibrary.Conv_IntToDouble` (`self.Duration`)))
    (set `self.NeedsToRun` false)))

(event `RemoveLives`
  (params (WasEaten :type Boolean))
  ;[1 1 1] Remove Lives
  (if (and WasEaten (> (`self.Lives`) 0))
    (set `self.Lives` (- (`self.Lives`) 1))))

(event `self.ReceiveBeginPlay`
  (bind _returnvalue (`GameplayStatics.GetPlayerCharacter` 0))
  ;[1 1 1] Respawn Player
  (bind _aspacman_game (cast `/Game/blueprint/PacmanGame` (`GameplayStatics.GetGameMode`)))
  (`self.PlayIntroMusic` _aspacman_game)
  (`/Engine/EditorBlueprintResources/StandardMacros.IsValid` _returnvalue :!label _label
    (:`Is Valid`
      (bind _aspacman_character (cast `/Game/blueprint/pacman_character` _returnvalue))
      (add `self.OnDestroyed` _aspacman_character (delegate `OnDestroyed_Event_0`)))))

(event `Respawn`
  ;[1 1 1] Respawn Player
  (goto _label))

(event `OnDestroyed_Event_0` :!signature `self.OnDestroyed`
  (params (DestroyedActor :type "Actor Object Reference"))
  ;[1 1 1] Respawn Player
  (`KismetSystemLibrary.Delay` 2.0)
  (if (> (`self.Lives`) 0)
    (bind _returnvalue (`|SpawnActorFromClass` "/Game/blueprint/pacman_character.pacman_character_C" (`self.Spawn Transform`) "Undefined" "OverrideRootScale" null null))
    (`Controller.Possess` (`GameplayStatics.GetPlayerController` 0) _returnvalue)
    (`self.Respawn`)
    (else
      (`GameplayStatics.OpenLevel` (`self.EndScreen`)))))

(event `DisablePlayerInput`
  (bind _returnvalue (`GameplayStatics.GetPlayerCharacter` 0))
  ;[1 1 1] Disable Players Input
  (`/Engine/EditorBlueprintResources/StandardMacros.IsValid` _returnvalue
    (:`Is Valid`
      (`self.DisableInput` _returnvalue null))))

(event `ActivateEnemiesAndPlayersMovement`
  ;[1 1 1] Activate Enemy
  (bind _outactors (`GameplayStatics.GetAllActorsOfClass` "/Game/blueprint/AI/Enemy_Character.Enemy_Character_C"))
  (for _array_element _outactors
    (set `/Game/blueprint/AI/Enemy_Character.Active` true _array_element))
  (for _array_element_2 _outactors
    (`Controller.Possess` (`self.GetInstigatorController` _array_element_2) _array_element_2)))

(event `EnablePlayerInput`
  (bind _returnvalue (`GameplayStatics.GetPlayerCharacter` 0))
  ;[1 1 1] Enable Players Input
  (`/Engine/EditorBlueprintResources/StandardMacros.IsValid` _returnvalue
    (:`Is Valid`
      (`self.EnableInput` _returnvalue null))))

(fn `UserConstructionScript`)
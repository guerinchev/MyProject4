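; Enemy character Blueprint for a Pac-Man game that kills the player on contact.
; A sphere attached to the mesh detects Pac-Man overlaps and, unless the game mode's NeedsToRun flag is set, plays the death sound and destroys him.
; It then removes a life through the game mode and holds the PacmanDied flag true briefly.
; A helper function sets the enemy's maximum walk speed.
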(event `self.Sphere.OnComponentBeginOverlap`
  (params (OverlappedComponent :type "PrimitiveComponent Object Reference") (OtherActor :type "Actor Object Reference") (OtherComp :type "PrimitiveComponent Object Reference") (OtherBodyIndex :type Integer) (bFromSweep :type Boolean) (SweepResult :type "HitResult Structure (by ref)"))
  ;[1 1 1] Eating Pacman
  (bind _aspacman_character (cast `/Game/blueprint/pacman_character` OtherActor))
  (bind _aspacman_game (cast `/Game/blueprint/PacmanGame` (`GameplayStatics.GetGameMode`)))
  (if (not (`/Game/blueprint/PacmanGame.NeedsToRun` _aspacman_game))
    (`GameplayStatics.PlaySound2D` "/Game/audio/pacman_dying.pacman_dying" 1.0 1.0 0.0 null null)
    (`self.K2_DestroyActor` _aspacman_character)
    (bind _aspacman_game_2 (cast `/Game/blueprint/PacmanGame` (`GameplayStatics.GetGameMode`)))
    (set `/Game/blueprint/PacmanGame.PacmanDied` true _aspacman_game_2)
    (`/Game/blueprint/PacmanGame.RemoveLives` _aspacman_game true)
    (`KismetSystemLibrary.Delay` 2.0)
    (set `/Game/blueprint/PacmanGame.PacmanDied` false _aspacman_game_2)))

(fn `Update Walk Speed`
  (params (`New Walk Speed` :type "Float (double-precision)"))
  (set `CharacterMovementComponent.MaxWalkSpeed` `New Walk Speed` (`self.CharacterMovement`)))

(fn `UserConstructionScript`
  (`SceneComponent.K2_AttachToComponent` (`self.Sphere`) (`self.Mesh`) "None" "KeepRelative" "KeepRelative" "KeepRelative" true))
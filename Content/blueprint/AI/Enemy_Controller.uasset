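; Enemy AI controller for a Pac-Man style game that runs patrol and player-detection logic for Enemy_Character.
; On possess, an active enemy starts BT_Enemy and copies its patrol path's looping flag to the Blackboard.
; Perception of the player stores them as the target, granting line of sight unless the game mode says NeedsToRun.
; Other perception updates start a timer that clears line of sight and target when it expires.
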(event `self.ReceivePossess`
  (params (PossessedPawn :type "Pawn Object Reference"))
  ;[1 1 1] Patrolling
  (bind _asenemy_character (cast `/Game/blueprint/AI/Enemy_Character` (`self.K2_GetPawn`)))
  (if (`/Game/blueprint/AI/Enemy_Character.Active` _asenemy_character)
    (`self.RunBehaviorTree` "/Game/blueprint/AI/BT_Enemy.BT_Enemy")
    (bind _asenemy_character_2 (cast `/Game/blueprint/AI/Enemy_Character` (`self.K2_GetPawn`)))
    (bind _output_get (set `self.MyPawn` _asenemy_character_2))
    (bind _patrolpath (`/Game/blueprint/AI/Enemy_Character.PatrolPath` _output_get))
    (`/Engine/EditorBlueprintResources/StandardMacros.IsValid` _patrolpath
      (:`Is Valid`
        (`BlackboardComponent.SetValueAsBool` (`AIBlueprintHelperLibrary.GetBlackboard` null) "PathLooping" (`/Game/blueprint/AI/PatrolPath.IsLooping` _patrolpath))))))

(event `self.AIPerception.OnTargetPerceptionUpdated`
  (params (Actor :type "Actor Object Reference") (Stimulus :type "AIStimulus Structure"))
  (bind _blackboard (`self.Blackboard`))
  ;[1 1 1] Determine Line of Site etc
  (if (and (`self.ActorHasTag` Actor "Player") (`.bSuccessfullySensed` (break `AIStimulus` Stimulus)))
    (`KismetSystemLibrary.K2_ClearAndInvalidateTimerHandle` (`self.EnemyTimer`))
    (bind _aspacman_game (cast `/Game/blueprint/PacmanGame` (`GameplayStatics.GetGameMode`)))
    (`BlackboardComponent.SetValueAsBool` _blackboard (`self.HasLineOfSight`) (== (`/Game/blueprint/PacmanGame.NeedsToRun` _aspacman_game) (`self.False`)))
    (`BlackboardComponent.SetValueAsObject` _blackboard (`self.EnemyActor`) Actor)
    (else
      (bind _returnvalue (`KismetSystemLibrary.K2_SetTimerDelegate` (delegate `StartEnemyTimer`) (`self.Line Of Sight Timer`)))
      (set `self.EnemyTimer` _returnvalue))))

(event `StartEnemyTimer`
  (bind _blackboard (`self.Blackboard`))
  ;[1 1 1] Determine Line of Site etc
  (`BlackboardComponent.SetValueAsBool` _blackboard (`self.HasLineOfSight`) false)
  (`BlackboardComponent.SetValueAsObject` _blackboard (`self.EnemyActor`) null))

(fn `UserConstructionScript`)
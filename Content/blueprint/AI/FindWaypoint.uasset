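; FindWaypoint is a behavior tree task that selects the enemy's current patrol waypoint.
; It reads the path index from the blackboard, converts that PatrolPath point to world space with the path actor's transform and writes it to the path vector key.
; It then updates the Enemy_Character walk speed and finishes successfully.
; A failed cast or invalid PatrolPath leaves the task unfinished, as neither branch calls FinishExecute.
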(event `self.ReceiveExecuteAI`
  (params (OwnerController :type "AIController Object Reference") (ControlledPawn :type "Pawn Object Reference"))
  (bind _asenemy_character (cast `/Game/blueprint/AI/Enemy_Character` ControlledPawn))
  (bind _patrolpath (`/Game/blueprint/AI/Enemy_Character.PatrolPath` _asenemy_character)
    (:`then`
      (`BTFunctionLibrary.SetBlackboardValueAsVector` (`self.BB_PathVector`) (`KismetMathLibrary.TransformLocation` (`Actor.GetTransform` _patrolpath) (`|GetArrayItem` (`/Game/blueprint/AI/PatrolPath.PatrolPoints` _patrolpath) (`BTFunctionLibrary.GetBlackboardValueAsInt` (`self.BB_PathIndex`)))))
      (`/Game/blueprint/AI/Enemy_Character.Update Walk Speed` _asenemy_character (`self.Walk Speed`))
      (`self.FinishExecute` true))
    (:`else`)))